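; PlayerBoat is the player-controlled boat, driven by throttle and steering axes with mouse look on the controller.
; Forward input accelerates a clamped speed, which decays at half acceleration toward the minimum without input.
; Steering eases yaw speed toward its target with FInterpTo.
; Each tick, MoveBoat applies both speeds as unswept local offset and rotation, without physics, and zeroes control-rotation roll.
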(event `self.ReceiveTick`
  (params (DeltaSeconds :type "Float (single-precision)"))
  (`self.MoveBoat` DeltaSeconds))

(event `InputAxis|MoveForward`
  (params (AxisValue :type "Float (single-precision)"))
  (`self.GetForwardSpeed` AxisValue))

(event `InputAxis|MoveRight`
  (params (AxisValue :type "Float (single-precision)"))
  (`self.GetSteeringSpeed` AxisValue))

(event `InputAxis|Turn`
  (params (AxisValue :type "Float (single-precision)"))
  (`self.AddControllerYawInput` (* AxisValue (`self.MouseSensivity`))))

(event `InputAxis|LookUp`
  (params (AxisValue :type "Float (single-precision)"))
  (`self.AddControllerPitchInput` (* AxisValue (`self.MouseSensivity`))))

(fn `GetForwardSpeed`
  (params (AxisValue :type "Float (double-precision)"))
  (bind _accelerationforce (`self.AccelerationForce`))
  (set `self.CurrentForwardSpeed` (`KismetMathLibrary.FClamp` (+ (`self.CurrentForwardSpeed`) (* (`KismetMathLibrary.SelectFloat` (* AxisValue _accelerationforce) (* _accelerationforce -0.5) (!= AxisValue 0.0)) (`GameplayStatics.GetWorldDeltaSeconds`))) (`self.MinSpeed`) (`self.MaxSpeed`))))

(fn `GetSteeringSpeed`
  (params (AxisValue :type "Float (double-precision)"))
  (set `self.CurrentYawSpeed` (`KismetMathLibrary.FInterpTo` (`self.CurrentYawSpeed`) (* AxisValue (`self.TurnSpeed`)) (`GameplayStatics.GetWorldDeltaSeconds`) 2.0)))

(fn `MoveBoat`
  (params (A :type "Float (double-precision)"))
  (bind (_returnvalue_roll _returnvalue_pitch _returnvalue_yaw) (`KismetMathLibrary.BreakRotator` (`self.GetControlRotation`)))
  (`self.K2_AddActorLocalOffset` (`KismetMathLibrary.MakeVector` (* A (`self.CurrentForwardSpeed`))))
  (`self.K2_AddActorLocalRotation` (`KismetMathLibrary.MakeRotator` 0.0 0.0 (* (`GameplayStatics.GetWorldDeltaSeconds`) (`self.CurrentYawSpeed`))))
  (`Controller.SetControlRotation` (`GameplayStatics.GetPlayerController` 0) (`KismetMathLibrary.MakeRotator` 0.0 _returnvalue_pitch _returnvalue_yaw)))

(fn `UserConstructionScript`)